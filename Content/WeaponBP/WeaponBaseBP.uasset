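; Base weapon Blueprint that detects and applies the player's melee hits on enemies, with damage, energy and combo stats built in its construction script.
; HitEnemy sphere-traces from DamagePoint, skipping enemies already hit until ClearHitedEnemy empties the list.
; New hits trigger player life steal, damage, particles, sound and camera shake.
; Brief time dilation adds impact, with a separate wait on combo index 3, and bosses also get a bone-shake reaction.
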(event `self.ReceiveBeginPlay`
  (`/Game/MeshMaterialFadeComp/MeshMaterialFadeComp.ResetFadeValue(StaticMesh)` (`self.MeshMaterialFadeComp`)))

(fn `ClearHitedEnemy`
  (if (> (`KismetArrayLibrary.Array_Length` (`self.HitedActor`)) 0)
    (`KismetArrayLibrary.Array_Clear` (`self.HitedActor`))))

(fn `HitEnemy`
  (locals (TempPlayer :type "/Game/player/Player_Bp Object Reference") (AttackHitTimeDilation :type "Float (double-precision)" :default 0.4) (NormalWaitDuration :type "Float (double-precision)" :default 0.05) (HardWaitTime :type "Float (double-precision)" :default 0.07) (TempHitActor :type "Actor Object Reference") (ImpactPoint :type "Vector Structure"))
  (bind _weapondata_damage (break `/Game/WeaponBP/WeaponData` (`self.WeaponData`)))
  ;[0 0 0 1 30] Sphere trace to detect is enemy or breakable object
  (bind (_outhit _havehit) (`self.TraceDetect`))
  (if _havehit
    (bind (_bblockinghit _binitialoverlap _time _distance _location _impactpoint _normal _impactnormal _physmat _hitactor) (`GameplayStatics.BreakHitResult` _outhit))
    (if (`self.ActorHasTag` _hitactor "Enemy")
      (if (not (`KismetArrayLibrary.Array_Contains` (`self.HitedActor`) _hitactor))
        (set `local.TempHitActor` _hitactor)
        (`KismetArrayLibrary.Array_Add` (`self.HitedActor`) _hitactor)
        (set `local.ImpactPoint` _impactpoint)
        (`|ExecutionSequence`
          (:`then_0`
            (bind _asplayer_bp (cast `/Game/player/Player_Bp` (`GameplayStatics.GetPlayerPawn` 0)))
            (bind _output_get (set `local.TempPlayer` _asplayer_bp))
            (`/Game/player/Player_Bp.LifeStealCheck` _output_get))
          (:`then_1`
            ;[0 0 0 1 30] Enemy take damage delegate
            (message `/Game/Enemy/ITakeDamage.TakeDamage` (`local.TempHitActor`) _weapondata_damage 0.0)
            ;[0 0 0 1 30] Spawn hit particle
            (`GameplayStatics.SpawnEmitterAtLocation` "/Game/All_Particles/FXVarietyPack/Particles/P_ky_hit1.P_ky_hit1" (`local.ImpactPoint`) (struct) (0.2 0.2 0.2))
            ;[0 0 0 1 30] Play hit sound
            (`GameplayStatics.PlaySound2D` "/Game/All_Sounds/PlayerSounds/Used/Hit_Cue.Hit_Cue" (`BigProjectGameInstance.GameSoundEffectMagnitude` (`/Game/player/Player_Bp.MainGameInstance` (`local.TempPlayer`))) 1.0 0.0 null null)
            ;[0 0 0 1 20] Camera shaking
            (`/Game/player/Player_Bp.AttackShakeSetting` (`local.TempPlayer`))
            (if (== (`/Game/player/Player_Bp.ComboIndex` (`local.TempPlayer`)) 3)
              ;[0 0 0 1 30] Slow time to increase attack feeling
              (`BigProjectFunctionLib.StartAttackHitTimeSlow` self (`local.AttackHitTimeDilation`) (`local.HardWaitTime`))
              (else
                (`BigProjectFunctionLib.StartAttackHitTimeSlow` self (`local.AttackHitTimeDilation`) (`local.NormalWaitDuration`)))))
          (:`then_2`
            (if (`self.ActorHasTag` (`local.TempHitActor`) "Boss")
              ;[0 0 0 1 30] Hit part bone shake(Boss only)
              (bind _asboss_re (cast `/Game/Enemy/Boss/Boss_Re` (`local.TempHitActor`)))
              (`/Game/Enemy/Boss/Boss_Re.BoneRotateDelegate` _asboss_re (`KismetSystemLibrary.GetDisplayName` (`local.TempHitActor`))))))))))

(fn `TraceDetect`
  (returns (OutHit :type "HitResult Structure") (HaveHit :type Boolean))
  (bind _returnvalue (`SceneComponent.K2_GetComponentLocation` (`self.DamagePoint`)))
  (bind (_outhit _returnvalue_2) (`KismetSystemLibrary.SphereTraceSingleForObjects` _returnvalue (+ _returnvalue (* (`SceneComponent.GetUpVector` (`self.DamagePoint`)) 100.0)) 20.0 (`|MakeArray` "ObjectTypeQuery3" "ObjectTypeQuery6" :!type "EObjectTypeQuery Enum") false (`|MakeArray` (`GameplayStatics.GetPlayerPawn` 0) :!type "Actor Object Reference") "None" true (struct :`R` 1.0 :`A` 1.0) (struct :`G` 1.0 :`A` 1.0) 1.0))
  (return _outhit _returnvalue_2))

(fn `UserConstructionScript`
  (set `self.WeaponData` (make `/Game/WeaponBP/WeaponData` 20.0 15.0 50.0 1.1 2.0 true 20.0)))