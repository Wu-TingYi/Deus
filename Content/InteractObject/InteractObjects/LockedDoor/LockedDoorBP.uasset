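; LockedDoorBP is an interactable locked door that shows a message widget when the player interacts with it.
; A box collision shows the inherited interact prompt when the player overlaps and hides it on exit, with the prompt text set to "開啟" (Open).
; InteractEffect lazily creates and reuses the DoorMessage widget, then removes any prompt and clears its ShowInteractWidget timer.
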(event `self.ReceiveBeginPlay`
  (`parent.ReceiveBeginPlay`))

(event `/Game/InteractObject/InteractObjects/ItemsData/InteractInterface.InteractEffect`
  (`self.DoorMessageWidget`
    (:`then`
      _)
    (:`else`
      (bind _returnvalue (`|CreateWidget` "/Game/UI/DoorMessage/DoorMessage.DoorMessage_C"))
      (bind _output_get (set `self.DoorMessageWidget` _returnvalue))))
  (`UserWidget.AddToViewport` _output_get 0)
  (bind _interactwordwidget (`self.InteractWordWidget`)
    (:`then`
      (`Widget.RemoveFromParent` _interactwordwidget)
      (`KismetSystemLibrary.K2_ClearTimer` self "ShowInteractWidget"))
    (:`else`)))

(event `self.BoxCollision.OnComponentBeginOverlap`
  (params (OverlappedComponent :type "PrimitiveComponent Object Reference") (OtherActor :type "Actor Object Reference") (OtherComp :type "PrimitiveComponent Object Reference") (OtherBodyIndex :type Integer) (bFromSweep :type Boolean) (SweepResult :type "HitResult Structure (by ref)"))
  ;[0 0 0 1 30] Overlap to show interact word
  (if (`self.ActorHasTag` OtherActor "Player")
    (`self.ShowInteractWidget`)))

(event `self.BoxCollision.OnComponentEndOverlap`
  (params (OverlappedComponent :type "PrimitiveComponent Object Reference") (OtherActor :type "Actor Object Reference") (OtherComp :type "PrimitiveComponent Object Reference") (OtherBodyIndex :type Integer))
  ;[0 0 0 1 30] End overlap to remove word
  (if (== OtherActor (`GameplayStatics.GetPlayerCharacter` 0))
    (`self.UnShowInteractWidget`)))

(fn `UserConstructionScript`
  (`parent.UserConstructionScript`)
  (set `self.InteractText` "開啟"))